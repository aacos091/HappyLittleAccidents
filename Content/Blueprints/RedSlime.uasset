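; RedSlime is a shootable target that awards score when a matching red projectile hits it.
; Its TriggerBox overlap casts the other actor to RedProjectile and compares that projectile's ColorEnum with its own.
; On a match, it adds ScoreValue to the Score on player 0's FirstPersonCharacter, then destroys itself.
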(event `self.TriggerBox.OnComponentBeginOverlap`
  (params (OverlappedComponent :type "PrimitiveComponent Object Reference") (OtherActor :type "Actor Object Reference") (OtherComp :type "PrimitiveComponent Object Reference") (OtherBodyIndex :type Integer) (bFromSweep :type Boolean) (SweepResult :type "HitResult Structure (by ref)"))
  ;[1 1 1] This checks to see if the correct projectile hit the slime, then destroys itself if it is true
  (bind _asred_projectile (cast `/Game/Projectiles/RedProjectile` OtherActor))
  (if (`|EnumEquality` (`/Game/Projectiles/RedProjectile.ColorEnum` _asred_projectile) (`self.ColorEnum`))
    (bind _asfirst_person_character (cast `/Game/Blueprints/FirstPersonCharacter` (`GameplayStatics.GetPlayerCharacter` 0)))
    (set `/Game/Blueprints/FirstPersonCharacter.Score` (+ (`/Game/Blueprints/FirstPersonCharacter.Score` _asfirst_person_character) (`self.ScoreValue`)) _asfirst_person_character)
    (`self.K2_DestroyActor`)))

(fn `UserConstructionScript`)