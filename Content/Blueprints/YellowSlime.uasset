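; YellowSlime is an enemy that moves along X and is killed by a matching colored projectile.
; From BeginPlay, a latent loop repeatedly moves its skeletal mesh toward relative X MoveForwardDistance, with a short delay between moves.
; When a YellowProjectile with the same ColorEnum overlaps its TriggerBox, it plays a death sound, adds ScoreValue to the FirstPersonCharacter's Score and destroys itself.
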(event `self.ReceiveBeginPlay`
  (bind _skeletalmeshcomponent (`self.SkeletalMeshComponent`))
  (bind (_relativelocation_x _relativelocation_y _relativelocation_z) (`KismetMathLibrary.BreakVector` (`SceneComponent.RelativeLocation` _skeletalmeshcomponent)))
  ;[1 1 1] Move forward rate
  (`KismetSystemLibrary.MoveComponentTo` _skeletalmeshcomponent (`KismetMathLibrary.MakeVector` (`self.MoveForwardDistance`) _relativelocation_y _relativelocation_z) (`SceneComponent.RelativeRotation` _skeletalmeshcomponent) false false 4.0 :!label _label)
  (`KismetSystemLibrary.Delay` 0.1)
  (goto _label))

(event `self.TriggerBox.OnComponentBeginOverlap`
  (params (OverlappedComponent :type "PrimitiveComponent Object Reference") (OtherActor :type "Actor Object Reference") (OtherComp :type "PrimitiveComponent Object Reference") (OtherBodyIndex :type Integer) (bFromSweep :type Boolean) (SweepResult :type "HitResult Structure (by ref)"))
  ;[1 1 1] This checks to see if the correct projectile hit the slime, then destroys itself if it is true
  (bind _asyellow_projectile (cast `/Game/Projectiles/YellowProjectile` OtherActor))
  (if (`|EnumEquality` (`/Game/Projectiles/YellowProjectile.ColorEnum` _asyellow_projectile) (`self.ColorEnum`))
    (`GameplayStatics.PlaySoundAtLocation` "/Game/Audio/EnemyDeathTest.EnemyDeathTest" (`SceneComponent.K2_GetComponentLocation` (`self.SkeletalMeshComponent`)) (struct) 1.0 1.0 0.0 null null null)
    (bind _asfirst_person_character (cast `/Game/Blueprints/FirstPersonCharacter` (`GameplayStatics.GetPlayerCharacter` 0)))
    (set `/Game/Blueprints/FirstPersonCharacter.Score` (+ (`/Game/Blueprints/FirstPersonCharacter.Score` _asfirst_person_character) (`self.ScoreValue`)) _asfirst_person_character)
    (`self.K2_DestroyActor`)))

(fn `UserConstructionScript`)