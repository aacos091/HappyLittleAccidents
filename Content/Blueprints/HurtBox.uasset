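; HurtBox is a trigger Blueprint that costs the player health when an enemy, such as a slime, enters it.
; On Box overlap, it compares the other actor's exact class against each entry in EnemyClasses.
; A match subtracts one Health from the player's FirstPersonCharacter, fetched by casting player character 0, then destroys the enemy.
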(event `self.Box.OnComponentBeginOverlap`
  (params (OverlappedComponent :type "PrimitiveComponent Object Reference") (OtherActor :type "Actor Object Reference") (OtherComp :type "PrimitiveComponent Object Reference") (OtherBodyIndex :type Integer) (bFromSweep :type Boolean) (SweepResult :type "HitResult Structure (by ref)"))
  (for _array_element (`self.EnemyClasses`)
    ;[1 1 1] Decrease health when slime crosses health
    (if (== _array_element (`GameplayStatics.GetObjectClass` OtherActor))
      (bind _asfirst_person_character (cast `/Game/Blueprints/FirstPersonCharacter` (`GameplayStatics.GetPlayerCharacter` 0)))
      (set `/Game/Blueprints/FirstPersonCharacter.Health` (- (`/Game/Blueprints/FirstPersonCharacter.Health` _asfirst_person_character) 1) _asfirst_person_character)
      (`self.K2_DestroyActor` OtherActor))))

(fn `UserConstructionScript`)