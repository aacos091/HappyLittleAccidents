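; SpawnBox is a spawner actor that keeps spawning random enemies at points marked by its arrow components.
; The construction script gathers nine arrows into SpawnLoc, and SpawnEnemy picks a random EnemiesArray class and arrow location, using a fixed rotation instead of the arrow's.
; After a start delay, BeginPlay loops SpawnEnemy indefinitely, waiting a random whole number of seconds between the min and max delay variables.
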(event `self.ReceiveBeginPlay`
  (`KismetSystemLibrary.Delay` (`self.StartSpawnDelay`))
  (`self.SpawnEnemy` :!label _label)
  (`KismetSystemLibrary.RetriggerableDelay` (`KismetMathLibrary.Conv_IntToDouble` (`KismetMathLibrary.RandomIntegerInRange` (`KismetMathLibrary.FTrunc` (`self.SpawnMoreDelayMin`)) (`KismetMathLibrary.FTrunc` (`self.SpawnMoreDelayMax`)))))
  (goto _label))

(fn `SpawnEnemy`
  (bind _enemiesarray (`self.EnemiesArray`))
  (bind _spawnloc (`self.SpawnLoc`))
  (`|SpawnActorFromClass` (`|GetArrayItem` _enemiesarray (`KismetMathLibrary.RandomInteger` (`KismetArrayLibrary.Array_Length` _enemiesarray))) (`KismetMathLibrary.MakeTransform` (`SceneComponent.K2_GetComponentLocation` (`|GetArrayItem` _spawnloc (`KismetMathLibrary.RandomInteger` (`KismetArrayLibrary.Array_Length` _spawnloc)))) (struct :`Yaw` 90.0)) "Undefined" "OverrideRootScale" null null))

(fn `UserConstructionScript`
  (bind _spawnloc (`self.SpawnLoc`))
  (bind _spawnloc_2 (`self.SpawnLoc`))
  (bind _spawnloc_3 (`self.SpawnLoc`))
  (`KismetArrayLibrary.Array_Add` _spawnloc_2 (`self.Arrow`))
  (`KismetArrayLibrary.Array_Add` _spawnloc_2 (`self.Arrow1`))
  (`KismetArrayLibrary.Array_Add` _spawnloc_2 (`self.Arrow2`))
  (`KismetArrayLibrary.Array_Add` _spawnloc_3 (`self.Arrow3`))
  (`KismetArrayLibrary.Array_Add` _spawnloc_3 (`self.Arrow4`))
  (`KismetArrayLibrary.Array_Add` _spawnloc_3 (`self.Arrow5`))
  (`KismetArrayLibrary.Array_Add` _spawnloc (`self.Arrow6`))
  (`KismetArrayLibrary.Array_Add` _spawnloc (`self.Arrow7`))
  (`KismetArrayLibrary.Array_Add` _spawnloc (`self.Arrow8`)))